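; Game mode for an egg-catching game that holds health, score and egg timing, and owns the HUD.
; BeginPlay creates the HUD and resets the game values.
; Tick halves the egg time value whenever score reaches a threshold, which then doubles, so difficulty ramps up.
; EndGameEvent disables player input, fades the camera, removes the HUD and, after a delay, shows the end-game widget with UI-only input.
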(event `EndGameEvent`
  (bind _returnvalue (`GameplayStatics.GetPlayerController` 0))
  (`self.DisableInput` (`GameplayStatics.GetPlayerCharacter` 0) (`GameplayStatics.GetPlayerController` 0))
  (`PlayerCameraManager.StartCameraFade` :`self` (`GameplayStatics.GetPlayerCameraManager` 0) :`ToAlpha` 0.8 :`Duration` 3.0 :`bHoldWhenFinished` true)
  (`Widget.RemoveFromParent` (`self.HeadsUpDisplay`))
  (`KismetSystemLibrary.Delay` 2.0)
  (bind _returnvalue_2 (`|CreateWidget` "/Game/Blueprints/Widgets/EndGameWidget.EndGameWidget_C"))
  (`UserWidget.AddToViewport` _returnvalue_2 0)
  (`WidgetBlueprintLibrary.SetInputMode_UIOnlyEx` _returnvalue _returnvalue_2)
  (set `PlayerController.bShowMouseCursor` true _returnvalue))

(event `self.ReceiveBeginPlay`
  (bind _returnvalue (`|CreateWidget` "/Game/Blueprints/HUD/HeadUpDisplay.HeadUpDisplay_C"))
  (bind _output_get (set `self.HeadsUpDisplay` _returnvalue))
  (`UserWidget.AddToViewport` _output_get 0)
  (set `self.Health` 3)
  (set `self.GameScore` 0)
  (set `self.SpeedAccumulator` 5)
  (set `self.EggTimeSpeed` 8.0))

(event `self.ReceiveTick`
  (params (DeltaSeconds :type "Float (single-precision)"))
  (if (>= (`self.GameScore`) (`self.SpeedAccumulator`))
    (set `self.SpeedAccumulator` (* (`self.SpeedAccumulator`) 2))
    (set `self.EggTimeSpeed` (/ (`self.EggTimeSpeed`) 2.0))))

(fn `Init Time`
  (set `self.EggTimeSpeed` 8.0))

(fn `UserConstructionScript`)