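; Egg spawner actor that periodically spawns eggs at its own transform in an egg-catching game.
; BeginPlay starts a looping timer at the SpawnDelay interval.
; Each tick of the timer casts the game mode to EggCatcherGameMode and, while its Health is above zero, spawns an EggBP, passing it the TriggerBox reference, and prints a debug message.
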(event `self.ReceiveBeginPlay`
  (`KismetSystemLibrary.K2_SetTimerDelegate` (delegate `OnTimer`) (`self.SpawnDelay`) true))

(event `OnTimer`
  (bind _asegg_catcher_game_mode (cast `/Game/EggCatcherGameMode` (`GameplayStatics.GetGameMode`)))
  (if (> (`/Game/EggCatcherGameMode.Health` _asegg_catcher_game_mode) 0)
    (`|SpawnActorFromClass` "/Game/Blueprints/EggBP.EggBP_C" (`self.GetTransform`) "Undefined" "OverrideRootScale" null (`self.TriggerBox`) null)
    (`KismetSystemLibrary.PrintString` "Egg Has Spawned")))

(fn `UserConstructionScript`)