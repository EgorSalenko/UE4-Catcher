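; BucketCharacter is a bucket actor that the player moves between four corner positions.
; BeginPlay enables input from player 0, and four diagonal input actions each set the actor's location to that of the matching referenced platform actor.
; Moves are instant jumps without sweep, except Up_Right, which sweeps and also prints a debug "Hello".
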(event `self.ReceiveBeginPlay`
  (`self.EnableInput` (`GameplayStatics.GetPlayerController` 0)))

(event `InputAction|Up_Right`
  (params (Key :type "Key Structure"))
  (:`Pressed`
    (`KismetSystemLibrary.PrintString` "Hello")
    (`self.K2_SetActorLocation` (`self.K2_GetActorLocation` (`self.Right Up Platform`)) true)))

(event `InputAction|Down_Right`
  (params (Key :type "Key Structure"))
  (:`Pressed`
    (`self.K2_SetActorLocation` (`self.K2_GetActorLocation` (`self.Right Down Platform`)))))

(event `InputAction|Down_Left`
  (params (Key :type "Key Structure"))
  (:`Pressed`
    (`self.K2_SetActorLocation` (`self.K2_GetActorLocation` (`self.Left Down Platform`)))))

(event `InputAction|Up_Left`
  (params (Key :type "Key Structure"))
  (:`Pressed`
    (`self.K2_SetActorLocation` (`self.K2_GetActorLocation` (`self.Left Up Platform`)))))

(fn `UserConstructionScript`)