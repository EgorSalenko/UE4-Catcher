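; EggManger is a spawner actor for an egg catcher game that periodically spawns EggBP actors at its own transform.
; On BeginPlay it caches the EggCatcherGameMode, calls its InitTime and starts a looping timer with a random start delay and a random interval, rolled once.
; Each tick of that timer spawns an egg while the game mode's Health is above zero, passing itself as the egg's manager.
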(event `self.ReceiveBeginPlay`
  (bind _asegg_catcher_game_mode (cast `/Game/Blueprints/EggCatcherGameMode` (`GameplayStatics.GetGameMode`)))
  (bind _output_get (set `self.GameModeRef` _asegg_catcher_game_mode))
  (`/Game/Blueprints/EggCatcherGameMode.Init Time` _output_get)
  (set `self.TimeLooping` true)
  (`KismetSystemLibrary.K2_SetTimerDelegate` (delegate `OnTimer`) (`KismetMathLibrary.RandomFloatInRange` 5.0 12.0) (`self.TimeLooping`) (`KismetMathLibrary.RandomFloatInRange` 5.0 8.5)))

(event `OnTimer`
  (if (> (`/Game/Blueprints/EggCatcherGameMode.Health` (`self.GameModeRef`)) 0)
    (`|SpawnActorFromClass` "/Game/Blueprints/EggBP.EggBP_C" (`self.GetTransform`) "Undefined" "OverrideRootScale" null self null)))

(fn `UserConstructionScript`)